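; Flying enemy actor that moves in a straight line along negative world X and explodes on overlap.
; BeginPlay picks a random integer multiplier to set its speed vector.
; Tick adds that vector to its location without sweep or delta-time scaling, so speed depends on frame rate.
; Overlapping any actor spawns an explosion particle effect at its location and destroys it.
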(event `self.ReceiveActorBeginOverlap`
  (params (OtherActor :type "Actor Object Reference"))
  ;[1 1 1] al generar un overlap se crea un efecto de particulas
  (`GameplayStatics.SpawnEmitterAtLocation` "/Game/Particles/P_Explosion.P_Explosion" (`self.K2_GetActorLocation`))
  (`self.K2_DestroyActor`))

(event `self.ReceiveTick`
  (params (DeltaSeconds :type "Float (single-precision)"))
  ;[1 1 1] agrega movimiento al objeto
  (`self.K2_SetActorLocation` (+ (`self.K2_GetActorLocation`) (`self.RandomEnemySpeed`))))

(event `self.ReceiveBeginPlay`
  ;[1 1 1] Genera velocidad de movimiento aleatoria para el objeto
  (set `self.RandomEnemySpeed` (* (`KismetMathLibrary.Conv_DoubleToVector` (`KismetMathLibrary.Conv_IntToDouble` (`KismetMathLibrary.RandomIntegerInRange` 1 3))) (-20.0 0.0 0.0))))

(fn `UserConstructionScript`)